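; Editor-facing actor that drives a graph grammar generator and draws the resulting graph as debug shapes.
; Reset seeds the graph with two connected nodes, and ReloadRules reloads the generator's rule set.
; ApplyRule applies one random rule and re-renders through the graph renderer, while Clear removes the debug shapes.
; All event and construction logic is empty, so everything runs through these functions.
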(fn `ApplyRule`
  (`GraphGeneratorComponent.ApplyRandomRule` (`self.GraphGenerator`))
  (`GraphRendererComponent.RenderGraph` (`self.GraphRenderer`)))

(fn `Clear`
  (`GraphRendererComponent.ClearDebugShapes` (`self.GraphRenderer`)))

(fn `ReloadRules`
  (`GraphGeneratorComponent.LoadRules` (`self.GraphGenerator`)))

(fn `Reset`
  (bind _nodes (`Graph.Nodes` (`self.Graph`)))
  (`self.ResetGraph`)
  (`Graph.AddNode` (`self.Graph`) (0.0 0.0))
  (`Graph.AddNode` (`self.Graph`) (200.0 0.0))
  (`Graph.AddEdge` (`self.Graph`) (`|GetArrayItem` _nodes) (`|GetArrayItem` _nodes 1)))

(fn `UserConstructionScript`)